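; Farmer AI character that performs plow, water, sow and harvest jobs on a target parcel.
; A job marks it unavailable, moves it to the parcel, then plays the matching montage through a server-to-multicast event chain.
; Water, sow and harvest also fire notification calls when the montage is requested.
; Montage completion, handled inside the multicast, applies the action or water to the parcel and frees the farmer.
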(event `PerformActinoOnParcel`
  (params (SelectedAction :type "/Game/Enums/EActionType Enum" :default "NewEnumerator0") (TargetParcel :type "/Game/Blueprints/Actors/BP_Parcel Object Reference"))
  (`/Engine/EditorBlueprintResources/StandardMacros.IsValid` TargetParcel
    (:`Is Valid`
      (set `self.IsAvailable` false)
      (bind _output_get (set `self.Target Parcel` TargetParcel))
      (`|AIMoveTo` self (`self.K2_GetActorLocation` _output_get) null
        (:`OnSuccess`
          (switch `/Game/Enums/EActionType` SelectedAction
            (:`NewEnumerator0`
              (`self.Server_PerformAction` "/Game/Character/Farmer/Animations/AM_Plowing.AM_Plowing"))
            (:`NewEnumerator1`
              (`self.Server_PerformAction` "/Game/Character/Farmer/Animations/AM_Watering.AM_Watering" "NewEnumerator1")
              (`self.OnWateringPerformed` (`self.WaterGived`)))
            (:`NewEnumerator2`
              (`self.Server_PerformAction` "/Game/Character/Farmer/Animations/AM_Sowing.AM_Sowing" "NewEnumerator2")
              (`self.OnSowingPerformed`))
            (:`NewEnumerator3`
              (`self.Server_PerformAction` "/Game/Character/Farmer/Animations/AM_Harvesting.AM_Harvesting" "NewEnumerator3")
              (`self.OnHarvestingPerformed`))))))))

(event `Server_PerformAction`
  (params (MontageToPlay :type "AnimMontage Object Reference") (ActionPerformed :type "/Game/Enums/EActionType Enum" :default "NewEnumerator0"))
  (`self.Multicast_PerformAction` MontageToPlay ActionPerformed))

(event `Multicast_PerformAction`
  (params (MontageToPlay :type "AnimMontage Object Reference") (ActionPerformed :type "/Game/Enums/EActionType Enum" :default "NewEnumerator0"))
  (`|PlayMontage` (`self.Mesh`) MontageToPlay
    (:`OnCompleted`
      (bind _target_parcel (`self.Target Parcel`)
        (:`then`
          (if (`|EnumEquality` ActionPerformed "NewEnumerator1")
            (`/Game/Blueprints/Actors/BP_Parcel.ReceiveWater` _target_parcel (`self.WaterGived`))
            (else
              (`/Game/Blueprints/Actors/BP_Parcel.ReceiveAction` _target_parcel ActionPerformed)))
          (set `self.IsAvailable` true))
        (:`else`)))))

(fn `UserConstructionScript`)
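; Farm game mode that builds the parcel grid on BeginPlay and spawns the farmer AI just above the first parcel.
; NotifyFarmer forwards a selected action and target parcel to the farmer only when it is available, returning whether it was dispatched.
; It binds to the farmer's watering, sowing and harvesting events and rebroadcasts them through its own dispatchers, acting as a relay between the farmer and listeners.
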(event `NotifyWateringPerformed`
  (params (WaterAmount :type Integer))
  (`self.OnWateringPerformed` WaterAmount))

(event `self.ReceiveBeginPlay`
  (bind (_firstparcellocation_x _firstparcellocation_y _firstparcellocation_z) (`KismetMathLibrary.BreakVector` (`self.FirstParcelLocation`)))
  (`|ExecutionSequence`
    (:`then_0`
      (`/Game/Blueprints/ActorComponents/AC_ParcelGridGenerator.GenerateGrid` (`self.AC_ParcelGridGenerator`) (`self.ParcelClass`) (`self.RowsNum`) (`self.ColumnsNum`) (`self.FirstParcelLocation`)))
    (:`then_1`
      (bind _returnvalue (`|SpawnActorFromClass` "/Game/Blueprints/Character/BP_FarmerAI.BP_FarmerAI_C" (`KismetMathLibrary.MakeTransform` (`KismetMathLibrary.MakeVector` _firstparcellocation_x _firstparcellocation_y (+ _firstparcellocation_z 35.0))) "AlwaysSpawn" "MultiplyWithRoot" null null))
      (set `self.FarmerAI` _returnvalue)
      (`|ExecutionSequence`
        (:`then_0`
          (add `/Game/Blueprints/Character/BP_FarmerAI.OnWateringPerformed` (`self.FarmerAI`) (delegate `NotifyWateringPerformed`)))
        (:`then_1`
          (add `/Game/Blueprints/Character/BP_FarmerAI.OnSowingPerformed` (`self.FarmerAI`) (delegate `NotifySowingPerformed`)))
        (:`then_2`
          (add `/Game/Blueprints/Character/BP_FarmerAI.OnHarvestingPerformed` (`self.FarmerAI`) (delegate `NotifyHarvestingPerformed`)))))))

(event `NotifySowingPerformed`
  (`self.OnSowingPerformed`))

(event `NotifyHarvestingPerformed`
  (`self.OnHarvestingPerformed`))

(fn `NotifyFarmer`
  (params (SelectedAction :type "/Game/Enums/EActionType Enum" :default "NewEnumerator0") (TargetParcel :type "/Game/Blueprints/Actors/BP_Parcel Object Reference"))
  (returns (IsFarmerAvailable :type Boolean))
  (bind _farmerai (`self.FarmerAI`)
    (:`then`
      (if (`/Game/Blueprints/Character/BP_FarmerAI.IsAvailable` _farmerai)
        (`/Game/Blueprints/Character/BP_FarmerAI.PerformActinoOnParcel` _farmerai SelectedAction TargetParcel)
        (return true)
        (else
          (return false))))
    (:`else`)))

(fn `UserConstructionScript`)
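; Player controller for a farming game, handling mouse interaction with parcels and the farm HUD on a fixed camera view.
; Holding left-click shows parcel info with timer-driven local countdowns for harvest time and water.
; Right-click opens an action menu gated by parcel state and pawn resources; selections go to the GameMode, showing a message if the farmer is unavailable.
; Cursor traces update the current parcel through a server event, and FarmPawn has a RepNotify.
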(event `self.ReceiveBeginPlay`
  (bind _actionsmenuwidget (`self.ActionsMenuWidget`))
  (`|ExecutionSequence`
    (:`then_0`
      ;[1 1 1 1 26] Init UI
      (if (`self.IsLocalController`)
        (`|ExecutionSequence`
          (:`then_0`
            (bind _returnvalue (`|CreateWidget` "/Game/UI/WBP_ActionsMenu.WBP_ActionsMenu_C"))
            (set `self.ActionsMenuWidget` _returnvalue)
            (bind _returnvalue_2 (`|CreateWidget` "/Game/UI/WBP_ParcelInfo.WBP_ParcelInfo_C"))
            (set `self.ParcelInfoWidget` _returnvalue_2)
            (bind _returnvalue_3 (`|CreateWidget` "/Game/UI/WBP_Messages.WBP_Messages_C"))
            (set `self.MessagesWidget` _returnvalue_3))
          (:`then_1`
            (`UserWidget.AddToViewport` _actionsmenuwidget 0)
            (`UserWidget.AddToViewport` (`self.ParcelInfoWidget`) 0)
            (`UserWidget.AddToViewport` (`self.MessagesWidget`) 0)
            (`Widget.SetVisibility` _actionsmenuwidget "Hidden")
            (`Widget.SetVisibility` (`self.ParcelInfoWidget`) "Hidden")
            (`Widget.SetVisibility` (`self.MessagesWidget`) "Hidden")))))
    (:`then_1`
      (bind _asbp_farm_game_mode (cast `/Game/Blueprints/Game/BP_FarmGameMode` (`GameplayStatics.GetGameMode`)))
      (set `self.FarmGameMode` _asbp_farm_game_mode))
    (:`then_2`
      (bind _returnvalue_4 (`GameplayStatics.GetActorOfClass` "/Script/Engine.CameraActor"))
      (`self.SetViewTargetWithBlend` _returnvalue_4))
    (:`then_3`
      (bind _actionsmenuwidget_2 (`self.ActionsMenuWidget`)
        (:`then`
          (add `/Game/UI/WBP_ActionsMenu.OnActionSelected` _actionsmenuwidget_2 (delegate `OnActionSelectedEvent`)))
        (:`else`)))))

(event `OnActionSelectedEvent`
  (params (ActionSelected :type "/Game/Enums/EActionType Enum" :default "NewEnumerator0"))
  (bind _currenthitparcel (`self.CurrentHitParcel`)
    (:`then`
      (bind _farmgamemode (`self.FarmGameMode`)
        (:`then`
          (bind _isfarmeravailable (`/Game/Blueprints/Game/BP_FarmGameMode.NotifyFarmer` _farmgamemode ActionSelected _currenthitparcel))
          (if (not _isfarmeravailable)
            (`self.SetMessageText` "The Farmer Is Not Available Right Now")))
        (:`else`)))
    (:`else`)))

(event `self.ReceivePossess`
  (params (PossessedPawn :type "Pawn Object Reference"))
  (`/Engine/EditorBlueprintResources/ActorMacros.Switch Has Authority`
    (:`Authority`
      (bind _asbp_farm_pawn (cast `/Game/Blueprints/Player/BP_FarmPawn` PossessedPawn))
      (set `self.FarmPawn` _asbp_farm_pawn))))

(event `UpdateRemainingTimeToHarvest`
  (bind _remaining_time_to_harvest (`self.Remaining Time to Harvest`))
  ;[1 1 1] Update Parcel Info in Widget
  (if (> _remaining_time_to_harvest 0)
    (bind _result (`/Engine/EditorBlueprintResources/StandardMacros.DecrementInt` _remaining_time_to_harvest)
      (:`  `
        (`/Game/UI/WBP_ParcelInfo.SetTimeToHarvestText` (`self.ParcelInfoWidget`) _result)))
    (else
      (`KismetSystemLibrary.K2_ClearAndInvalidateTimerHandle` (`self.UpdateRemainingTimeToHarvestHandle`)))))

(event `Key|LeftMouseButton`
  (params (Key :type "Key Structure"))
  ;[1 1 1 1 28] Mouse Click Events
  (:`Pressed`
    (bind _hitparcel (`self.GetHitParcel`))
    (`/Engine/EditorBlueprintResources/StandardMacros.IsValid` _hitparcel
      (:`Is Valid`
        (bind _parcelinfowidget (`self.ParcelInfoWidget`)
          (:`then`
            (`/Game/UI/WBP_ParcelInfo.SetIsPlowedText` _parcelinfowidget (`/Game/Blueprints/Actors/BP_Parcel.IsPlowed` _hitparcel))
            (`Widget.SetVisibility` _parcelinfowidget "Visible")
            ;[1 1 1] Update Parcel Info in Widget
            (`|ExecutionSequence`
              (:`then_0`
                (bind _output_get (set `self.Remaining Time to Harvest` (`/Game/Blueprints/Actors/BP_Parcel.RemainingTimeToHarvest` _hitparcel)))
                (`/Game/UI/WBP_ParcelInfo.SetTimeToHarvestText` (`self.ParcelInfoWidget`) _output_get)
                (bind _returnvalue (`KismetSystemLibrary.K2_SetTimerDelegate` (delegate `UpdateRemainingTimeToHarvest`) 1.0 true))
                (set `self.UpdateRemainingTimeToHarvestHandle` _returnvalue))
              (:`then_1`
                (bind _output_get_2 (set `self.Current Water` (`/Game/Blueprints/Actors/BP_Parcel.CurrentWater` _hitparcel)))
                (`/Game/UI/WBP_ParcelInfo.SetCurrentWaterText` (`self.ParcelInfoWidget`) _output_get_2)
                (bind _timetoupdatewater (`/Game/Blueprints/Actors/BP_Parcel.TimeToUpdateWater` _hitparcel))
                (bind _returnvalue_2 (`KismetSystemLibrary.K2_SetTimerDelegate` (delegate `UpdateRemainigWater`) _timetoupdatewater true _timetoupdatewater))
                (set `self.UpdateCurrentWaterHandle` _returnvalue_2))))
          (:`else`)))))
  (:`Released`
    (bind _parcelinfowidget_2 (`self.ParcelInfoWidget`)
      (:`then`
        (`Widget.SetVisibility` _parcelinfowidget_2 "Hidden")
        (`KismetSystemLibrary.K2_ClearAndInvalidateTimerHandle` (`self.UpdateRemainingTimeToHarvestHandle`))
        (`KismetSystemLibrary.K2_ClearAndInvalidateTimerHandle` (`self.UpdateCurrentWaterHandle`)))
      (:`else`))))

(event `UpdateRemainigWater`
  (bind _current_water (`self.Current Water`))
  ;[1 1 1] Update Parcel Info in Widget
  (if (> _current_water 0)
    (`/Engine/EditorBlueprintResources/StandardMacros.DecrementInt` _current_water
      (:`  `
        (`/Game/UI/WBP_ParcelInfo.SetCurrentWaterText` (`self.ParcelInfoWidget`) 0)
        (`KismetSystemLibrary.K2_ClearAndInvalidateTimerHandle` (`self.UpdateCurrentWaterHandle`))))))

(event `Key|RightMouseButton`
  (params (Key :type "Key Structure"))
  ;[1 1 1 1 28] Mouse Click Events
  (:`Pressed`
    (bind _hitparcel (`self.GetHitParcel`))
    (`/Engine/EditorBlueprintResources/StandardMacros.IsValid` _hitparcel
      (:`Is Valid`
        (bind _actionsmenuwidget (`self.ActionsMenuWidget`)
          (:`then`
            (`self.SetActionsAvailability` _hitparcel)
            (`Widget.SetVisibility` _actionsmenuwidget "Visible"))
          (:`else`))))))

(event `Server_UpdateCurrentHitParcel`
  (params (CurrentHitParcel :type "/Game/Blueprints/Actors/BP_Parcel Object Reference"))
  (set `self.CurrentHitParcel` CurrentHitParcel))

(event `SetMessageText`
  (params (Text :type Text))
  (bind _messageswidget (`self.MessagesWidget`)
    (:`then`
      (`/Game/UI/WBP_Messages.SetMessageText` _messageswidget Text)
      (`Widget.SetVisibility` _messageswidget "Visible")
      (`KismetSystemLibrary.Delay` (`self.MessageDisplayingTime`))
      (`Widget.SetVisibility` _messageswidget "Hidden"))
    (:`else`)))

(fn `GetHitParcel`
  (returns (HitParcel :type "/Game/Blueprints/Actors/BP_Parcel Object Reference"))
  (bind _asbp_parcel (cast `/Game/Blueprints/Actors/BP_Parcel` (`.HitActor` (`GameplayStatics.BreakHitResult` (`self.GetHitResultUnderCursorForObjects` (`self.ObjectTypes`) false))))
    (:`then`
      (`self.Server_UpdateCurrentHitParcel` _asbp_parcel)
      (return _asbp_parcel))
    (:`CastFailed`
      (`self.Server_UpdateCurrentHitParcel` null)
      (return null))))

(fn `OnRep_FarmPawn`
  (`/Engine/EditorBlueprintResources/ActorMacros.Switch Has Authority`
    (:`Remote`
      (`/Engine/EditorBlueprintResources/StandardMacros.IsValid` (`self.FarmPawn`)
        (:`Is Not Valid`
          (bind _asbp_farm_pawn (cast `/Game/Blueprints/Player/BP_FarmPawn` (`self.K2_GetPawn`)))
          (set `self.FarmPawn` _asbp_farm_pawn))))))

(fn `SetActionsAvailability`
  (params (TargetParcel :type "/Game/Blueprints/Actors/BP_Parcel Object Reference"))
  (locals (HasSufficientSeeds :type Boolean) (IsPlantGrowing :type Boolean) (InParcel :type "/Game/Blueprints/Actors/BP_Parcel Object Reference"))
  (set `local.InParcel` TargetParcel)
  (bind _actionsmenuwidget (`self.ActionsMenuWidget`)
    (:`then`
      (`|ExecutionSequence`
        (:`then_0`
          (`Widget.SetIsEnabled` (`/Game/UI/WBP_ActionsMenu.Btn_Plow` _actionsmenuwidget) (not (`/Game/Blueprints/Actors/BP_Parcel.IsPlowed` (`local.InParcel`)))))
        (:`then_1`
          (bind _farmpawn (`self.FarmPawn`)
            (:`then`
              (`Widget.SetIsEnabled` (`/Game/UI/WBP_ActionsMenu.Btn_Water` _actionsmenuwidget) (> (`/Game/Blueprints/Player/BP_FarmPawn.Water` _farmpawn) 0)))
            (:`else`)))
        (:`then_2`
          (bind _farmpawn_2 (`self.FarmPawn`)
            (:`then`
              (set `local.HasSufficientSeeds` (> (`/Game/Blueprints/Player/BP_FarmPawn.Seeds` _farmpawn_2) 0))
              (`Widget.SetIsEnabled` (`/Game/UI/WBP_ActionsMenu.Btn_Sow` _actionsmenuwidget) (and (not (`/Game/Blueprints/Actors/BP_Parcel.IsOccupiedByPlant` (`local.InParcel`))) (`local.HasSufficientSeeds`) (`/Game/Blueprints/Actors/BP_Parcel.IsPlowed` (`local.InParcel`)))))
            (:`else`)))
        (:`then_3`
          (`Widget.SetIsEnabled` (`/Game/UI/WBP_ActionsMenu.Btn_Harvest` _actionsmenuwidget) (`/Game/Blueprints/Actors/BP_Parcel.IsHarvestable` (`local.InParcel`))))))
    (:`else`)))

(fn `UserConstructionScript`)
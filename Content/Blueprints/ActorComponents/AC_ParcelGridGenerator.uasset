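; Actor component that spawns a grid of parcel actors from a given class, row and column count, and first location.
; GenerateGrid loops over rows along Y and columns along X, offsetting each spawn by the parcel size.
; Any parcel size still at zero is measured from the spawned actor's bounds and stored, so the first parcel sets the spacing for the rest.
; Only X and Y positions are set.
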(fn `GenerateGrid`
  (params (ActorToSpawn :type "Actor Class Reference") (RowsNum :type Integer) (ColumnsNum :type Integer) (FirsLocation :type "Vector Structure"))
  (locals (ParcelXSize :type "Float (double-precision)") (ParcelYSize :type "Float (double-precision)") (ActorClass :type "Actor Class Reference"))
  (set `local.ActorClass` ActorToSpawn)
  (for _index (range RowsNum)
    (for _index_2 (range ColumnsNum)
      (bind _returnvalue (`|SpawnActorFromClass` (`local.ActorClass`) (`KismetMathLibrary.MakeTransform` (`KismetMathLibrary.MakeVector` (+ (* (`local.ParcelXSize`) _index_2) (.x FirsLocation)) (+ (* _index (`local.ParcelYSize`)) (.y FirsLocation)))) "Undefined" "MultiplyWithRoot" null null))
      (`|ExecutionSequence`
        (:`then_0`
          (if (== 0.0 (`local.ParcelXSize`))
            (bind (_origin _boxextent) (`Actor.GetActorBounds` _returnvalue false false))
            (set `local.ParcelXSize` (* (.x _boxextent) 2.0))))
        (:`then_1`
          (if (== (`local.ParcelYSize`) 0.0)
            (set `local.ParcelYSize` (* (.y _boxextent) 2.0))))))))
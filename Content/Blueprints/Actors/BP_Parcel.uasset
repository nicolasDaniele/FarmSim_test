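; Farm plot actor that can be plowed, sown, watered and harvested, and brightens on cursor hover.
; ReceiveAction and ReceiveWater drive its state, with looping timers draining water and counting growth down to harvestable, independently of each other.
; Water, occupancy, countdown and harvest reset replicate through Server-to-Multicast RPCs.
; A dynamic material instance swaps base and normal textures as the state changes.
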(event `self.ReceiveBeginPlay`
  (bind _plane (`self.Plane`))
  (bind _returnvalue (`PrimitiveComponent.CreateDynamicMaterialInstance` _plane 0 "/Game/Materials/M_ParcelBase.M_ParcelBase" "None"))
  (bind _output_get (set `self.DynamicMaterialInstance` _returnvalue))
  (`PrimitiveComponent.SetMaterial` _plane 0 _output_get))

(event `self.Box.OnBeginCursorOver`
  (params (TouchedComponent :type "PrimitiveComponent Object Reference"))
  ;[1 1 1] Mouse Hover
  (`MaterialInstanceDynamic.SetScalarParameterValue` (`self.DynamicMaterialInstance`) "Brightness" 3.0))

(event `self.Box.OnEndCursorOver`
  (params (TouchedComponent :type "PrimitiveComponent Object Reference"))
  ;[1 1 1] Mouse Hover
  (`MaterialInstanceDynamic.SetScalarParameterValue` (`self.DynamicMaterialInstance`) "Brightness" 1.0))

(event `Multicast_UpdateTexture`
  (params (Value :type "Texture Object Reference"))
  ;[1 1 1 1 28] RPCs
  (`MaterialInstanceDynamic.SetTextureParameterValue` (`self.DynamicMaterialInstance`) "BaseTexture" Value))

(event `OnPlowed`
  ;[1 1 1 1 26] Parcel State
  (set `self.IsPlowed` true)
  (`self.Multicast_UpdateTexture` "/Game/Textures/Parcel/Plowed/T_ParcelPlowed_Base.T_ParcelPlowed_Base")
  (`self.Multicast_UpdateNormal` "/Game/Textures/Parcel/NotPlowed/T_ParcelNotPlowed_Normal.T_ParcelNotPlowed_Normal"))

(event `OnWatered`
  (params (WaterAmount :type Integer))
  (bind _timetoupdatewater (`self.TimeToUpdateWater`))
  ;[1 1 1 1 26] Parcel State
  (`self.Server_UpdateCurrentWater` (+ WaterAmount (`self.CurrentWater`)))
  (bind _returnvalue (`KismetSystemLibrary.K2_SetTimerDelegate` (delegate `DecrementWater`) _timetoupdatewater true _timetoupdatewater))
  (set `self.WaterTimerHandle` _returnvalue))

(event `Multicast_UpdateNormal`
  (params (Value :type "Texture Object Reference"))
  ;[1 1 1 1 28] RPCs
  (`MaterialInstanceDynamic.SetTextureParameterValue` (`self.DynamicMaterialInstance`) "Normal" Value))

(event `DecrementWater`
  (bind _currentwater (`self.CurrentWater`))
  ;[1 1 1 1 26] Parcel State
  (if (> _currentwater 0)
    (`self.Server_UpdateCurrentWater` (- _currentwater 1))
    (else
      (`KismetSystemLibrary.K2_ClearAndInvalidateTimerHandle` (`self.WaterTimerHandle`)))))

(event `Server_UpdateCurrentWater`
  (params (CurrentWater :type Integer))
  ;[1 1 1 1 28] RPCs
  (`self.Multicast_UpdateCurrentWater` CurrentWater))

(event `Multicast_UpdateCurrentWater`
  (params (CurrentWater :type Integer))
  ;[1 1 1 1 28] RPCs
  (set `self.CurrentWater` CurrentWater))

(event `OnSowed`
  ;[1 1 1 1 26] Parcel State
  (`self.Server_UpdateIsOccupiedByPlant` true)
  (`self.Server_UpdateRemainingTimeToHarvest` (`self.TimeToHarvest`))
  (bind _returnvalue (`KismetSystemLibrary.K2_SetTimerDelegate` (delegate `OnPlanted`) 1.0 true 1.0))
  (set `self.GrowingPlantTimerHandle` _returnvalue))

(event `Server_UpdateRemainingTimeToHarvest`
  (params (RemainingTimeToHarvest :type Integer))
  ;[1 1 1 1 28] RPCs
  (`self.Multicast_UpdateRemainingTimeToHarvest` RemainingTimeToHarvest))

(event `OnPlanted`
  (bind _remainingtimetoharvest (`self.RemainingTimeToHarvest`))
  ;[1 1 1 1 26] Parcel State
  (if (> _remainingtimetoharvest 0)
    (`self.Server_UpdateRemainingTimeToHarvest` (- _remainingtimetoharvest 1))
    (else
      (set `self.IsHarvestable` true)
      (`KismetSystemLibrary.K2_ClearAndInvalidateTimerHandle` (`self.GrowingPlantTimerHandle`))
      (`self.Multicast_UpdateTexture` "/Game/Textures/Parcel/Harvestable/T_ParcelHarvestable_Base.T_ParcelHarvestable_Base")
      (`self.Multicast_UpdateNormal` "/Game/Textures/Parcel/Harvestable/T_ParcelHarvestable_Normal.T_ParcelHarvestable_Normal"))))

(event `Multicast_UpdateRemainingTimeToHarvest`
  (params (RemainingTimeToHarvest :type Integer))
  ;[1 1 1 1 28] RPCs
  (set `self.RemainingTimeToHarvest` RemainingTimeToHarvest))

(event `OnHarvested`
  ;[1 1 1 1 26] Parcel State
  (`self.Server_ResetState`))

(event `Server_UpdateIsOccupiedByPlant`
  (params (IsOccupiedByPlant :type Boolean))
  ;[1 1 1 1 28] RPCs
  (`self.Multicast__UpdateIsOccupiedByPlant` IsOccupiedByPlant))

(event `Multicast__UpdateIsOccupiedByPlant`
  (params (IsOccupiedByPlant :type Boolean))
  ;[1 1 1 1 28] RPCs
  (set `self.IsOccupiedByPlant` IsOccupiedByPlant))

(event `ReceiveAction`
  (params (ActionPerformed :type "/Game/Enums/EActionType Enum" :default "NewEnumerator0"))
  (bind _returnvalue (`KismetSystemLibrary.GetDisplayName` self))
  (switch `/Game/Enums/EActionType` ActionPerformed
    (:`NewEnumerator0`
      (`self.OnPlowed`)
      (`KismetSystemLibrary.PrintString` (`KismetStringLibrary.Concat_StrStr` _returnvalue " PLOWED") true true (struct :`R` 1.0 :`G` 0.85665 :`A` 1.0) 4.0))
    (:`NewEnumerator2`
      (`self.OnSowed`)
      (`KismetSystemLibrary.PrintString` (`KismetStringLibrary.Concat_StrStr` _returnvalue " SOWED") true true (struct :`R` 1.0 :`G` 0.85665 :`A` 1.0) 4.0))
    (:`NewEnumerator3`
      (`self.OnHarvested`)
      (`KismetSystemLibrary.PrintString` (`KismetStringLibrary.Concat_StrStr` _returnvalue " HARVESTED") true true (struct :`R` 1.0 :`G` 0.85665 :`A` 1.0) 4.0))))

(event `Server_ResetState`
  ;[1 1 1 1 28] RPCs
  (`self.Multicast_ResetState`))

(event `Multicast_ResetState`
  ;[1 1 1 1 28] RPCs
  (`self.ResetState`))

(event `ReceiveWater`
  (params (WaterAmount :type Integer))
  (`self.OnWatered` WaterAmount)
  (`KismetSystemLibrary.PrintString` (`KismetStringLibrary.Concat_StrStr` (`KismetSystemLibrary.GetDisplayName` self) " WATERED") true true (struct :`R` 1.0 :`G` 0.85665 :`A` 1.0) 4.0))

(fn `GetRemainingTimeToHarvest`
  (returns (ReturnValue :type "Float (single-precision)"))
  (bind _growingplanttimerhandle (`self.GrowingPlantTimerHandle`))
  (if (`KismetSystemLibrary.K2_IsValidTimerHandle` _growingplanttimerhandle)
    (return (`KismetSystemLibrary.K2_GetTimerRemainingTimeHandle` _growingplanttimerhandle))
    (else
      (return 0.0))))

(fn `ResetState`
  (set `self.IsPlowed` false)
  (set `self.CurrentWater` 0)
  (set `self.TimeToHarvest` 0)
  (set `self.IsHarvestable` false)
  (set `self.IsOccupiedByPlant` false)
  (`self.Multicast_UpdateTexture` "/Game/Textures/Parcel/NotPlowed/T_ParcelNotPlowed_Base.T_ParcelNotPlowed_Base")
  (`self.Multicast_UpdateNormal` "/Game/Textures/Parcel/NotPlowed/T_ParcelNotPlowed_Normal.T_ParcelNotPlowed_Normal"))

(fn `UserConstructionScript`)